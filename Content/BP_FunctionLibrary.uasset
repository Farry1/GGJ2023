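; Blueprint function library of shared helpers for a grid-based game, covering mouse picking, grid surface checks, input toggling and level reload.
; Mouse position comes from a deprojected cursor trace, returning a far-off sentinel location on a miss.
; Terrain and roots checks trace vertically through a grid instance's world position, each on its own trace channel.
; Other helpers test two group-type collections for overlap and set the player controller's input flag.
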(fn `CompareGridGroupType`
  (params (A :type "Array of EGridObjectGroup Enum") (B :type "Array of EGridObjectGroup Enum"))
  (returns (Result :type Boolean))
  (for _array_element A
    (if (`KismetArrayLibrary.Array_Contains` B _array_element)
      (return true)))
  (return false))

(fn `EnableInput`
  (params (WorldContext :type "Object Object Reference") (Enabled :type Boolean))
  (bind _asbp_player_controller (cast `/Game/Core/PlayerController/BP_PlayerController` (`GameplayStatics.GetPlayerController` WorldContext)))
  (set `/Game/Core/PlayerController/BP_PlayerController.bAllowInput` Enabled _asbp_player_controller))

(fn `Get Mouse Position`
  (returns (Location :type "Vector Structure") (ReturnValue :type Boolean))
  (bind (_worldlocation _worlddirection) (`PlayerController.DeprojectMousePositionToWorld` (`GameplayStatics.GetPlayerController` null)))
  (bind (_outhit _returnvalue) (`KismetSystemLibrary.LineTraceSingle` null _worldlocation (+ _worldlocation (* _worlddirection (10000.0 10000.0 10000.0))) "TraceTypeQuery3"))
  (if _returnvalue
    (return (`.Location` (`GameplayStatics.BreakHitResult` _outhit)) _returnvalue)
    (else
      (return (9999999.0 9999999.0 9999999.0) false))))

(fn `RaycastRootsAtGridPosition`
  (params (`World Context` :type "Object Object Reference") (InPoint :type "IntPoint Structure"))
  (returns (Result :type Boolean) (Location :type "Vector Structure"))
  (bind _returnvalue (`Grid.GetWorldPosition` (`StaticHelpers.GetGridInstance` `World Context`) InPoint))
  (bind (_outhit _returnvalue_2) (`KismetSystemLibrary.LineTraceSingle` :`WorldContextObject` `World Context` :`Start` (+ _returnvalue (0.0 0.0 500.0)) :`End` (+ _returnvalue (0.0 0.0 -500.0)) :`TraceChannel` "TraceTypeQuery4" :`DrawTime` 0.5))
  (return _returnvalue_2 (`.Location` (`GameplayStatics.BreakHitResult` _outhit))))

(fn `RaycastTerrainAtGridPosition`
  (params (`World Context` :type "Object Object Reference") (InPoint :type "IntPoint Structure"))
  (returns (Result :type Boolean) (Location :type "Vector Structure"))
  (bind _returnvalue (`Grid.GetWorldPosition` (`StaticHelpers.GetGridInstance` `World Context`) InPoint))
  (bind (_outhit _returnvalue_2) (`KismetSystemLibrary.LineTraceSingle` :`WorldContextObject` `World Context` :`Start` (+ _returnvalue (0.0 0.0 500.0)) :`End` (+ _returnvalue (0.0 0.0 -500.0)) :`TraceChannel` "TraceTypeQuery3" :`DrawTime` 0.5))
  (return _returnvalue_2 (`.Location` (`GameplayStatics.BreakHitResult` _outhit))))

(fn `ReloadLevel`
  (params (WorldContext :type "Object Object Reference"))
  (bind _returnvalue (`GameplayStatics.GetCurrentLevelName` WorldContext))
  (`GameplayStatics.OpenLevel` WorldContext (`KismetStringLibrary.Conv_StringToName` _returnvalue)))