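; BP_OverlapCheckComponent is an actor component that reports which actors overlap its owner's tagged sphere collision.
; On BeginPlay it finds the owner's component tagged OverlapSphere and stores it as a sphere component.
; GetOverlappingActors returns every actor overlapping that sphere except the owner, drawing a debug box above each one.
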(event `self.ReceiveBeginPlay`
  (bind _assphere_collision (cast `SphereComponent` (`|GetArrayItem` (`Actor.GetComponentsByTag` (`self.GetOwner`) "/Script/Engine.ActorComponent" "OverlapSphere"))))
  (set `self.SphereCollision` _assphere_collision))

(fn `GetOverlappingActors`
  (returns (Actors :type "Array of Actor Object Reference"))
  (locals (Result :type "Array of Actor Object Reference"))
  (bind _spherecollision (`self.SphereCollision`))
  (`/Engine/EditorBlueprintResources/StandardMacros.IsValid` _spherecollision
    (:`Is Valid`
      (for _array_element (`PrimitiveComponent.GetOverlappingActors` _spherecollision "/Script/Engine.Actor")
        (if (!= (`self.GetOwner`) _array_element)
          (`KismetSystemLibrary.DrawDebugBox` (+ (`Actor.K2_GetActorLocation` _array_element) (0.0 0.0 150.0)) (5.0 5.0 5.0) (struct :`G` 0.107181 :`B` 1.0 :`A` 1.0) (struct) 0.0 5.0)
          (`KismetArrayLibrary.Array_Add` (`local.Result`) _array_element)))
      (return (`local.Result`)))))