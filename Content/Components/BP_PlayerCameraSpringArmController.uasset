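; Player camera component that provides smoothed mouse wheel zoom by changing the length of its owner's spring arm.
; It finds the SpringArmComponent on BeginPlay and stores the inverted wheel axis as zoom input.
; Each Tick lerps toward that input using a delta-time-scaled dampening speed, then adds it, scaled by zoom speed, to the arm length, clamped between minimum and maximum camera heights.
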(event `self.ReceiveBeginPlay`
  (`parent.ReceiveBeginPlay`)
  (set `self.SpringArm` (`Actor.GetComponentByClass` (`self.GetOwner`) "/Script/Engine.SpringArmComponent")))

(event `self.ReceiveTick`
  (params (DeltaSeconds :type "Float (single-precision)"))
  (`parent.ReceiveTick` DeltaSeconds)
  (bind _output_get (set `self.CurrentMouseWheelInput` (`KismetMathLibrary.Lerp` (`self.CurrentMouseWheelInput`) (`self.MouseWheelInput`) (* (`self.ZoomDampeningSpeed`) DeltaSeconds))))
  (bind _output_get_2 (set `self.TargetHeightOffset` (* _output_get (`self.ZoomSpeed`))))
  (set `SpringArmComponent.TargetArmLength` (`KismetMathLibrary.FClamp` (+ (`SpringArmComponent.TargetArmLength` (`self.SpringArm`)) _output_get_2) (`self.MinCameraHeight`) (`self.MaxCameraHeight`)) (`self.SpringArm`)))

(event `InputAxisKey|MouseWheelAxis`
  (params (AxisValue :type "Float (single-precision)"))
  (set `self.MouseWheelInput` (* AxisValue -1.0)))