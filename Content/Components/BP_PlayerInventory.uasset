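; Player inventory component that stores items in an InventorySlots array and exposes functions to read and remove them.
; GetItems returns a filtered list containing only the valid slot entries.
; RemoveItem deletes the first matching entry by index, shrinking the array, then fires OnInventoryChanged and reports whether the removal succeeded.
; It has no active event logic and no function for adding items.
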(fn `GetItems`
  (returns (Result :type "Array of PlaceableObjectData Object Reference"))
  (locals (TempResult :type "Array of PlaceableObjectData Object Reference"))
  (for _array_element (`self.InventorySlots`)
    (`/Engine/EditorBlueprintResources/StandardMacros.IsValid` _array_element
      (:`Is Valid`
        (`KismetArrayLibrary.Array_Add` (`local.TempResult`) _array_element))))
  (return (`local.TempResult`)))

(fn `RemoveItem`
  (params (Data :type "PlaceableObjectData Object Reference"))
  (returns (Result :type Boolean))
  (bind _returnvalue (`KismetArrayLibrary.Array_Find` (`self.InventorySlots`) Data))
  (if (!= _returnvalue -1)
    (`KismetArrayLibrary.Array_Remove` (`self.InventorySlots`) _returnvalue)
    (`self.OnInventoryChanged` self)
    (return true)
    (else
      (return false))))