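; Progression component that tracks a point score and advances through an ordered array of tiers until the game is won.
; AddPoints accumulates the score and moves up at most one tier per call when the next tier's PointsNeeded is met.
; It broadcasts points scored, new tier reached, or game won, treating arrival at the last tier as the win.
; Helper functions expose the current and next tiers.
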(fn `AddPoints`
  (params (Points :type Integer))
  (bind _output_get (set `self.CurrentPoints` (+ (`self.CurrentPoints`) Points)))
  (if (>= _output_get (`ProgressionTierData.PointsNeeded` (`self.GetNextTier`)))
    (`/Engine/EditorBlueprintResources/StandardMacros.IncrementInt` (`self.CurrentTierIndex`)
      (:`  `
        (if (`self.HasWonGame?`)
          (`self.OnGameWon` (`self.CurrentPoints`))
          (else
            (`self.OnNewTierReached` (`|GetArrayItem` (`self.ProgressionTiers`) (`self.CurrentTierIndex`)) (`self.GetNextTier`) (`self.CurrentPoints`))))))
    (else
      (`self.OnPointsScored` (`self.CurrentPoints`)))))

(fn `GetCurrentAndNextTier`
  (returns (Current :type "ProgressionTierData Object Reference") (Next :type "ProgressionTierData Object Reference"))
  (locals (CurrentTier :type "ProgressionTierData Object Reference") (NextTier :type "ProgressionTierData Object Reference"))
  (set `local.CurrentTier` (`|GetArrayItem` (`self.ProgressionTiers`) (`self.CurrentTierIndex`)))
  (if (< (`self.CurrentTierIndex`) (`KismetArrayLibrary.Array_LastIndex` (`self.ProgressionTiers`)))
    (set `local.NextTier` (`|GetArrayItem` (`self.ProgressionTiers`) (+ (`self.CurrentTierIndex`) 1)))
    (return (`local.CurrentTier`) (`local.NextTier`))
    (else
      (return (`local.CurrentTier`) null))))

(fn `GetNextTier`
  (returns (NextTier :type "ProgressionTierData Object Reference"))
  (if (< (`self.CurrentTierIndex`) (`KismetArrayLibrary.Array_LastIndex` (`self.ProgressionTiers`)))
    (return (`|GetArrayItem` (`self.ProgressionTiers`) (+ (`self.CurrentTierIndex`) 1)))))

(fn `HasWonGame?`
  (returns (ReturnValue :type Boolean))
  (return (not (`KismetSystemLibrary.IsValid` (`self.GetNextTier`)))))