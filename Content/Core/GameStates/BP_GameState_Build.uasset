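; Game state for build mode, where the player positions, rotates and places a buildable grid object.
; On enter it spawns a preview from PlaceableData, which follows the mouse with grid snapping and a vertical trace for height.
; Tile changes and 90-degree rotations respawn indicators for valid and invalid tiles.
; Primary action removes the item from inventory and commits the object to the grid; cancelling destroys it, and both return to the default state.
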(event `self.EnterStateEvent`
  (`parent.EnterStateEvent`)
  (bind _returnvalue (`|SpawnActorFromClass` (`GridObjectData.BuildableClass` (`self.PlaceableData`)) (`KismetMathLibrary.MakeTransform` (`PlayerController.DeprojectMousePositionToWorld` (`GameplayStatics.GetPlayerController` 0))) "Undefined" "OverrideRootScale" null null))
  (bind _asbp_grid_object_base (cast `/Game/GridObjects/BP_GridObject_Base` _returnvalue))
  (set `self.PlaceableObject` _asbp_grid_object_base))

(event `self.ExitStateEvent`
  (bind _placeableobject (`self.PlaceableObject`))
  (`parent.ExitStateEvent`)
  (`self.ClearOwnTileIndicator`)
  (`/Engine/EditorBlueprintResources/StandardMacros.IsValid` _placeableobject
    (:`Is Valid`
      (`Actor.K2_DestroyActor` _placeableobject))))

(event `self.OnPrimaryAction`
  (bind _placeableobject (`self.PlaceableObject`))
  (if (and (`KismetSystemLibrary.IsValid` _placeableobject) (`.ReturnValue` (`GridObject.CanBePlaced` _placeableobject)))
    (bind _result (`/Game/Components/BP_PlayerInventory.RemoveItem` (`Actor.GetComponentByClass` (`GameplayStatics.GetPlayerController` 0) "/Game/Components/BP_PlayerInventory.BP_PlayerInventory_C") (`self.PlaceableData`)))
    (if _result
      (`GridObject.AddToGrid` (`self.PlaceableObject`))
      (`/Game/GridObjects/BP_GridObject_Base.OnBeingPlaced` (`self.PlaceableObject`))
      (set `self.PlaceableObject` null)
      (`self.EndGameState`)
      (else
        (`KismetSystemLibrary.PrintString` "Couldnt remove item. Something went wrong")))))

(event `self.OnCancel`
  (`self.EndGameState` :!label _label))

(event `self.OnSecondaryAction`
  (goto _label))

(event `self.OnRotateLeftAction`
  (`parent.OnRotateLeftAction`)
  (`self.Rotate` 90.0))

(event `self.OnRotateRightAction`
  (`parent.OnRotateRightAction`)
  (`self.Rotate` -90.0))

(event `self.TickStateEvent`
  (params (DeltaTime :type "Float (single-precision)"))
  (bind _returnvalue (`self.GetSnappedMousePosition`))
  (bind _output_get (set `self.CurrentGridIndex` (`Grid.GetGridPosition` (`StaticHelpers.GetGridInstance` self) _returnvalue)))
  (if (!= _output_get (`self.PreviousGridIndex`))
    (set `self.PreviousGridIndex` (`self.CurrentGridIndex`))
    (`Actor.K2_SetActorLocation` (`self.PlaceableObject`) _returnvalue false false)
    (`self.OnNewTileHovered`)))

(fn `ClearOwnTileIndicator`
  (for _array_element (`self.OwnTileIndicators`)
    (`/Engine/EditorBlueprintResources/StandardMacros.IsValid` _array_element
      (:`Is Valid`
        (`Actor.K2_DestroyActor` _array_element)))))

(fn `Close`
  (bind _returnvalue (`|GenericCreateObject` "/Game/Core/GameStates/BP_GameState_Default.BP_GameState_Default_C"))
  (bind _asbp_player_controller (cast `/Game/Core/PlayerController/BP_PlayerController` (`GameplayStatics.GetPlayerController` 0)))
  (`/Game/Core/PlayerController/BP_PlayerController.SwitchGameState` _asbp_player_controller _returnvalue))

(fn `EndGameState`
  (bind _placeableobject (`self.PlaceableObject`))
  (`/Engine/EditorBlueprintResources/StandardMacros.IsValid` _placeableobject
    (:`Is Valid`
      (`Actor.K2_DestroyActor` _placeableobject))
    (:`Is Not Valid`
      _))
  (`self.Close`))

(fn `GetMousePosition`)

(fn `GetSnappedMousePosition`
  (returns (ReturnValue :type "Vector Structure"))
  (locals (CurrentMousePosition :type "Vector Structure" :default (0.0 0.0 0.0)))
  (bind (_location _returnvalue) (`/Game/BP_FunctionLibrary.Get Mouse Position`))
  (bind _snappedmouseposition (`self.SnappedMousePosition`))
  (bind (_x _y) (`KismetMathLibrary.BreakVector3f` (`self.SnappedMousePosition`)))
  (if _returnvalue
    (bind _output_get (set `local.CurrentMousePosition` _location))
    (set `self.LastMousePosition` _output_get)
    (else
      (set `local.CurrentMousePosition` (`self.LastMousePosition`))))
  (set `self.SnappedMousePosition` (`KismetMathLibrary.Vector_SnappedToGrid` (`local.CurrentMousePosition`) 50.0))
  (bind _outhit (`KismetSystemLibrary.LineTraceSingle` (+ _snappedmouseposition (0.0 0.0 500.0)) (+ _snappedmouseposition (0.0 0.0 -500.0)) "TraceTypeQuery3"))
  (return (`KismetMathLibrary.MakeVector` _x _y (`.Z` (`KismetMathLibrary.BreakVector3f` (`.Location` (`GameplayStatics.BreakHitResult` _outhit)))))))

(fn `OnNewTileHovered`
  (locals (NewLocalVar_0 :type "Transform Structure"))
  (bind (_validtiles _invalidtiles) (`GridObject.CanBePlaced` (`self.PlaceableObject`)))
  (`self.ClearOwnTileIndicator`)
  (`/Engine/EditorBlueprintResources/StandardMacros.IsValid` (`self.PlaceableObject`)
    (:`Is Valid`
      (for _array_element _validtiles
        (`self.SpawnTileIndicatorAt` _array_element (struct :`G` 0.233997 :`B` 1.0 :`A` 1.0)))
      (for _array_element_2 _invalidtiles
        (`self.SpawnTileIndicatorAt` _array_element_2 (struct :`R` 1.0 :`B` 0.125658 :`A` 1.0))))))

(fn `Rotate`
  (params (Direction :type "Float (double-precision)"))
  (bind _placeableobject (`self.PlaceableObject`))
  (bind (_returnvalue_roll _returnvalue_pitch _returnvalue_yaw) (`KismetMathLibrary.BreakRotator` (`Actor.K2_GetActorRotation` (`self.PlaceableObject`))))
  (`/Engine/EditorBlueprintResources/StandardMacros.IsValid` _placeableobject
    (:`Is Valid`
      (`Actor.K2_SetActorRotation` _placeableobject (`KismetMathLibrary.MakeRotator` 0.0 0.0 (- _returnvalue_yaw Direction)) false)
      (`self.OnNewTileHovered`))))

(fn `SpawnTileIndicatorAt`
  (params (GridCoordinates :type "IntPoint Structure") (Color :type "LinearColor Structure"))
  (bind (_returnvalue_x _returnvalue_y _returnvalue_z) (`KismetMathLibrary.BreakVector` (`Actor.K2_GetActorLocation` (`self.PlaceableObject`))))
  (bind (_returnvalue_x_2 _returnvalue_y_2) (`KismetMathLibrary.BreakVector` (`Grid.GetWorldPosition` (`StaticHelpers.GetGridInstance` self) GridCoordinates)))
  (bind _returnvalue (`|SpawnActorFromClass` "/Game/UI/BP_GridIndicator.BP_GridIndicator_C" (`KismetMathLibrary.MakeTransform` (`KismetMathLibrary.MakeVector` _returnvalue_x_2 _returnvalue_y_2 _returnvalue_z)) "Undefined" "OverrideRootScale" null null))
  (`KismetArrayLibrary.Array_Add` (`self.OwnTileIndicators`) _returnvalue)
  (if (> (`KismetArrayLibrary.Array_Length` (`Grid.GetGridActorsAt` (`StaticHelpers.GetGridInstance` self) GridCoordinates)) 0)
    (`/Game/UI/BP_GridIndicator.SetColor` _returnvalue Color)))