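; Game state that scores a newly placed grid object against its neighbouring cells while card input is disabled.
; Delayed self-calling events step through cells, actors and matching group counts, each count spawning a flying indicator, wobbling the object and adding the neighbour's base score.
; Afterwards, a tier increase enables the new-card buttons; otherwise it switches to the Default state, or Lost if the inventory is empty.
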(event `self.EnterStateEvent`
  (`parent.EnterStateEvent`)
  (bind _asbp_player_controller (cast `/Game/Core/PlayerController/BP_PlayerController` (`GameplayStatics.GetPlayerController` 0)))
  (bind _output_get (set `self.Game UI` (`/Game/Core/PlayerController/BP_PlayerController.GameUI` _asbp_player_controller)))
  (`/Game/UI/WBP_GameUI.Disable Input On Cards` _output_get true)
  (`/Game/UI/WBP_GameUI.CardDeckAnimate` _output_get false)
  (bind _output_get_2 (set `self.BP Progression Component` (`/Game/Core/PlayerController/BP_PlayerController.BP_ProgressionComponent` _asbp_player_controller)))
  (set `self.InitialTier` (`/Game/Components/BP_ProgressionComponent.CurrentTierIndex` _output_get_2))
  (bind _returnvalue (`GridObject.GetNeighbouringCells` (`self.PlacedObject`)))
  (set `self.NeighbouringCells` _returnvalue)
  (`KismetSystemLibrary.Delay` 0.2)
  (`self.AddPointsForCell`))

(event `self.ExitStateEvent`
  (`parent.ExitStateEvent`))

(event `AddPointsForCell`
  (set `self.GridActorsIndex` 0)
  (if (<= (`self.NeighbouringCellIndex`) (`KismetArrayLibrary.Array_LastIndex` (`self.NeighbouringCells`)))
    (`KismetSystemLibrary.Delay` 0.2)
    (`self.CheckGridActors`)
    (else
      (`self.DoneScoring`))))

(event `CheckGridActors`
  (set `self.SingleItemStackSizeIndex` 0)
  (if (<= (`self.GridActorsIndex`) (`KismetArrayLibrary.Array_LastIndex` (`Grid.GetGridActorsAt` (`StaticHelpers.GetGridInstance` (`GameplayStatics.GetPlayerController` 0)) (`|GetArrayItem` (`self.NeighbouringCells`) (`self.NeighbouringCellIndex`)))))
    (`KismetSystemLibrary.Delay` 0.2)
    (`self.CheckSingleItemStackSize`)
    (else
      (`/Engine/EditorBlueprintResources/StandardMacros.IncrementInt` (`self.NeighbouringCellIndex`)
        (:`  `
          (`self.AddPointsForCell`))))))

(event `CheckSingleItemStackSize`
  (bind _gridobjectdata (`GridObject.GridObjectData` (`|GetArrayItem` (`Grid.GetGridActorsAt` (`StaticHelpers.GetGridInstance` (`GameplayStatics.GetPlayerController` 0)) (`|GetArrayItem` (`self.NeighbouringCells`) (`self.NeighbouringCellIndex`))) (`self.GridActorsIndex`))))
  (set `self.SingleItemMaxCount` 0)
  (for _array_element (`GridObjectData.MyGridObjectGroups` (`GridObject.GridObjectData` (`self.PlacedObject`)))
    (set `self.SingleItemMaxCount` (+ (`BlueprintMapLibrary.Map_Find` (`GridObjectData.GroupAndCount` _gridobjectdata) _array_element) (`self.SingleItemMaxCount`))))
  (if (< (`self.SingleItemStackSizeIndex`) (`self.SingleItemMaxCount`))
    (if true
      (`KismetSystemLibrary.Delay` 0.2)
      (bind _returnvalue (`|SpawnActorFromClass` "/Game/GridObjects/BP_CountIndicator.BP_CountIndicator_C" (`KismetMathLibrary.MakeTransform` (0.0 0.0 0.0)) "Undefined" "OverrideRootScale" null (`.Location` (`/Game/BP_FunctionLibrary.RaycastTerrainAtGridPosition` (`GameplayStatics.GetPlayerController` 0) (`|GetArrayItem` (`self.NeighbouringCells`) (`self.NeighbouringCellIndex`)))) (`Actor.K2_GetActorLocation` (`self.PlacedObject`)) null))
      (set `self.CalculatedTileIndicator` _returnvalue)
      (bind _asbp_grid_object_base (cast `/Game/GridObjects/BP_GridObject_Base` (`self.PlacedObject`))
        (:`then`
          (`/Game/GridObjects/BP_GridObject_Base.WobbleAnim` _asbp_grid_object_base))
        (:`CastFailed`
          _))
      (`/Game/Components/BP_ProgressionComponent.AddPoints` (`self.BP Progression Component`) (`GridObjectData.BaseScore` _gridobjectdata))
      (`KismetSystemLibrary.Delay` 0.25)
      (`/Engine/EditorBlueprintResources/StandardMacros.IncrementInt` (`self.SingleItemStackSizeIndex`)
        (:`  `
          (`self.CheckSingleItemStackSize`)))
      (else
        (`/Engine/EditorBlueprintResources/StandardMacros.IncrementInt` (`self.SingleItemStackSizeIndex`)
          (:`  `
            (`self.CheckSingleItemStackSize`)))))
    (else
      (`/Engine/EditorBlueprintResources/StandardMacros.IncrementInt` (`self.GridActorsIndex`)
        (:`  `
          (`KismetSystemLibrary.Delay` 0.2)
          (`self.CheckGridActors`))))))

(event `DoneScoring`
  (bind _game_ui (`self.Game UI`))
  (if (> (`/Game/Components/BP_ProgressionComponent.CurrentTierIndex` (`self.BP Progression Component`)) (`self.InitialTier`))
    (`/Game/UI/WBP_GameUI.EnableNewCardsButtons` (`self.Game UI`) true)
    (elif (> (`KismetArrayLibrary.Array_Length` (`/Game/Components/BP_PlayerInventory.GetItems` (`Actor.GetComponentByClass` (`GameplayStatics.GetPlayerController` 0) "/Game/Components/BP_PlayerInventory.BP_PlayerInventory_C"))) 0)
      (bind _returnvalue (`|GenericCreateObject` "/Game/Core/GameStates/BP_GameState_Default.BP_GameState_Default_C"))
      (bind _asbp_player_controller (cast `/Game/Core/PlayerController/BP_PlayerController` (`GameplayStatics.GetPlayerController` 0)))
      (`/Game/Core/PlayerController/BP_PlayerController.SwitchGameState` _asbp_player_controller _returnvalue)
      (`/Game/UI/WBP_GameUI.Disable Input On Cards` _game_ui false)
      (`/Game/UI/WBP_GameUI.CardDeckAnimate` _game_ui true)
      (else
        (bind _returnvalue_2 (`|GenericCreateObject` (`GameplayStatics.GetPlayerController` 0) "/Game/Core/GameStates/BP_GameState_Lost.BP_GameState_Lost_C"))
        (bind _asbp_player_controller_2 (cast `/Game/Core/PlayerController/BP_PlayerController` (`GameplayStatics.GetPlayerController` 0)))
        (`/Game/Core/PlayerController/BP_PlayerController.SwitchGameState` _asbp_player_controller_2 _returnvalue_2)))))