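; Game state that deals the current progression tier's cards into the player's inventory, with input disabled while it is active.
; Self-calling delayed events add each guaranteed card, then make as many random picks, repeats allowed, as the possible-card pool has entries.
; A failed add pauses longer, then moves on without retrying.
; When dealing ends, it switches the player controller to a new default game state.
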(event `self.EnterStateEvent`
  (bind _bp_progression_component (`self.BP Progression Component`))
  (`parent.EnterStateEvent`)
  (`/Game/BP_FunctionLibrary.EnableInput` (`GameplayStatics.GetPlayerController` 0))
  (bind _asbp_player_controller (cast `/Game/Core/PlayerController/BP_PlayerController` (`GameplayStatics.GetPlayerController` 0)))
  (bind _output_get (set `self.Game UI` (`/Game/Core/PlayerController/BP_PlayerController.GameUI` _asbp_player_controller)))
  (`/Game/UI/WBP_GameUI.Disable Input On Cards` _output_get true)
  (set `self.BP Player Inventory` (`/Game/Core/PlayerController/BP_PlayerController.BP_PlayerInventory` _asbp_player_controller))
  (set `self.BP Progression Component` (`/Game/Core/PlayerController/BP_PlayerController.BP_ProgressionComponent` _asbp_player_controller))
  (`KismetSystemLibrary.Delay` 1.0)
  (set `self.CurrentTier` (`|GetArrayItem` (`/Game/Components/BP_ProgressionComponent.ProgressionTiers` _bp_progression_component) (`/Game/Components/BP_ProgressionComponent.CurrentTierIndex` _bp_progression_component)))
  (`self.DealNextCardGuaranteed`))

(event `self.ExitStateEvent`
  (`parent.ExitStateEvent`)
  (`/Game/BP_FunctionLibrary.EnableInput` (`GameplayStatics.GetPlayerController` 0) true)
  (`/Game/UI/WBP_GameUI.Disable Input On Cards` (`self.Game UI`) false))

(event `DealNextCardGuaranteed`
  (if (<= (`self.GuaranteedIndex`) (`KismetArrayLibrary.Array_LastIndex` (`ProgressionTierData.GuaranteedCards` (`self.CurrentTier`))))
    (`KismetSystemLibrary.Delay` 0.1)
    (bind _result (`/Game/Components/BP_PlayerInventory.AddItem` (`self.BP Player Inventory`) (`|GetArrayItem` (`ProgressionTierData.GuaranteedCards` (`self.CurrentTier`)) (`self.GuaranteedIndex`))))
    (if (not _result)
      (`KismetSystemLibrary.Delay` 2.0))
    (`/Engine/EditorBlueprintResources/StandardMacros.IncrementInt` (`self.GuaranteedIndex`)
      (:`  `
        (`self.DealNextCardGuaranteed`)))
    (else
      (`self.DealNextCardRandom`))))

(event `DealNextCardRandom`
  (bind _possiblecards (`ProgressionTierData.PossibleCards` (`self.CurrentTier`)))
  (if (<= (`self.RandomIndex`) (`KismetArrayLibrary.Array_LastIndex` (`ProgressionTierData.PossibleCards` (`self.CurrentTier`))))
    (`KismetSystemLibrary.Delay` 0.1)
    (bind _result (`/Game/Components/BP_PlayerInventory.AddItem` (`self.BP Player Inventory`) (`|GetArrayItem` _possiblecards (`KismetMathLibrary.RandomIntegerInRange` 0 (`KismetArrayLibrary.Array_LastIndex` _possiblecards)))))
    (if (not _result)
      (`KismetSystemLibrary.Delay` 2.0))
    (`/Engine/EditorBlueprintResources/StandardMacros.IncrementInt` (`self.RandomIndex`)
      (:`  `
        (`self.DealNextCardRandom`)))
    (else
      (`KismetSystemLibrary.Delay` 0.25)
      (`self.CardDealingDone`))))

(event `CardDealingDone`
  (bind _returnvalue (`GameplayStatics.GetPlayerController` 0))
  (bind _returnvalue_2 (`|GenericCreateObject` _returnvalue "/Game/Core/GameStates/BP_GameState_Default.BP_GameState_Default_C"))
  (bind _asbp_player_controller (cast `/Game/Core/PlayerController/BP_PlayerController` _returnvalue))
  (`/Game/Core/PlayerController/BP_PlayerController.SwitchGameState` _asbp_player_controller _returnvalue_2))