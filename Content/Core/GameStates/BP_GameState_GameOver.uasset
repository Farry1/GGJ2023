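; Game-over state for the game's state system, run when a match ends.
; On entry it disables player input, animates the card deck in the game UI, hides that UI and starts a constant rotation on the player pawn.
; After a short delay it shows the end-game screen widget, passing it whether the player has won.
; Exit only runs the parent behavior.
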(event `self.EnterStateEvent`
  (`parent.EnterStateEvent`)
  (`/Game/BP_FunctionLibrary.EnableInput` (`GameplayStatics.GetPlayerController` 0))
  (bind _asbp_player_controller (cast `/Game/Core/PlayerController/BP_PlayerController` (`GameplayStatics.GetPlayerController` 0)))
  (`/Game/UI/WBP_GameUI.CardDeckAnimate` (`/Game/Core/PlayerController/BP_PlayerController.GameUI` _asbp_player_controller) false)
  (`/Game/Core/PlayerController/BP_PlayerController.HideGameUI` _asbp_player_controller)
  (bind _asbp_player_pawn (cast `/Game/Player/BP_PlayerPawn` (`GameplayStatics.GetPlayerPawn` 0)))
  (`/Game/Player/BP_PlayerPawn.ConstantRotation` _asbp_player_pawn)
  (`KismetSystemLibrary.Delay` 1.0)
  (bind _returnvalue (`|CreateWidget` "/Game/UI/WBP_EndGameScree.WBP_EndGameScree_C" (`GameplayStatics.GetPlayerController` 0) (`self.HasWon?`)))
  (`UserWidget.AddToViewport` _returnvalue 0))

(event `self.ExitStateEvent`
  (`parent.ExitStateEvent`))