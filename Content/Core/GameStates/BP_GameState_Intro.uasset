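; BP_GameState_Intro is the opening state in the game's state flow, playing a fade-in before card dealing begins.
; On enter, it holds the camera on black briefly, then fades the view in over a short timed sequence.
; It then has BP_PlayerController show the game UI, constructs a BP_GameState_DealCards object and switches to it, while exit only calls the parent.
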(event `self.EnterStateEvent`
  (bind _returnvalue (`GameplayStatics.GetPlayerCameraManager` 0))
  (`parent.EnterStateEvent`)
  (`PlayerCameraManager.SetManualCameraFade` :`self` _returnvalue :`InFadeAmount` 1.0)
  (`KismetSystemLibrary.Delay` 1.0)
  (`PlayerCameraManager.StartCameraFade` :`self` _returnvalue :`FromAlpha` 1.0 :`Duration` 2.0)
  (`KismetSystemLibrary.Delay` 2.0)
  (bind _asbp_player_controller (cast `/Game/Core/PlayerController/BP_PlayerController` (`GameplayStatics.GetPlayerController` 0)))
  (`/Game/Core/PlayerController/BP_PlayerController.CreateAndShowGameUI` _asbp_player_controller)
  (bind _returnvalue_2 (`|GenericCreateObject` _asbp_player_controller "/Game/Core/GameStates/BP_GameState_DealCards.BP_GameState_DealCards_C"))
  (`/Game/Core/PlayerController/BP_PlayerController.SwitchGameState` _asbp_player_controller _returnvalue_2))

(event `self.ExitStateEvent`
  (`parent.ExitStateEvent`))