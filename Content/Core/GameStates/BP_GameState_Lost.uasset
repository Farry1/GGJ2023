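; BP_GameState_Lost is the game state entered, by its name, when the player loses.
; On entering, it disables player input and calls CardDeckAnimate(false) on the player controller's game UI.
; It then starts the player pawn's ConstantRotation; exiting the state only runs the parent logic.
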(event `self.EnterStateEvent`
  (`parent.EnterStateEvent`)
  (`/Game/BP_FunctionLibrary.EnableInput` (`GameplayStatics.GetPlayerController` 0))
  (bind _asbp_player_controller (cast `/Game/Core/PlayerController/BP_PlayerController` (`GameplayStatics.GetPlayerController` 0)))
  (`/Game/UI/WBP_GameUI.CardDeckAnimate` (`/Game/Core/PlayerController/BP_PlayerController.GameUI` _asbp_player_controller) false)
  (bind _asbp_player_pawn (cast `/Game/Player/BP_PlayerPawn` (`GameplayStatics.GetPlayerPawn` 0)))
  (`/Game/Player/BP_PlayerPawn.ConstantRotation` _asbp_player_pawn))

(event `self.ExitStateEvent`
  (`parent.ExitStateEvent`))