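; BP_GameState_SwitchLevel is a game state that transitions to another level with a fade to black.
; On entering, it disables input, hides the game UI on BP_PlayerController and runs a two-second camera fade out.
; It then holds the screen black with a manual fade and opens the level held in its Level reference.
; Exiting only calls the parent logic.
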(event `self.EnterStateEvent`
  (`parent.EnterStateEvent`)
  (bind _asbp_player_controller (cast `/Game/Core/PlayerController/BP_PlayerController` (`GameplayStatics.GetPlayerController` 0)))
  (`/Game/BP_FunctionLibrary.EnableInput` self)
  (`/Game/Core/PlayerController/BP_PlayerController.HideGameUI` _asbp_player_controller)
  (bind _playercameramanager (`PlayerController.PlayerCameraManager` _asbp_player_controller))
  (`PlayerCameraManager.StartCameraFade` :`self` _playercameramanager :`FromAlpha` 0.0 :`ToAlpha` 1.0 :`Duration` 2.0)
  (`KismetSystemLibrary.Delay` 2.0)
  (`PlayerCameraManager.SetManualCameraFade` :`self` _playercameramanager :`InFadeAmount` 1.0)
  (`GameplayStatics.OpenLevelBySoftObjectPtr` (`self.Level`)))

(event `self.ExitStateEvent`
  (`parent.ExitStateEvent`))