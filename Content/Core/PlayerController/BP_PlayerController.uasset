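; Player controller that drives gameplay through a swappable game-state object, starting in BP_GameState_Intro with the mouse cursor shown.
; It uses a state pattern: SwitchGameState exits the old state and enters the new one, and OpenBuildMode switches to a build state with placeable data.
; Tick and input for primary, secondary, cancel and Q/E rotation are forwarded to the active state, with input gated by AllowInput.
; It also creates and removes the game UI widget.
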(event `self.ReceiveBeginPlay`
  (set `self.bShowMouseCursor` true)
  (bind _returnvalue (`|GenericCreateObject` "/Game/Core/GameStates/BP_GameState_Intro.BP_GameState_Intro_C"))
  (`self.SwitchGameState` _returnvalue))

(event `self.ReceiveTick`
  (params (DeltaSeconds :type "Float (single-precision)"))
  (`parent.ReceiveTick` DeltaSeconds)
  (`/Engine/EditorBlueprintResources/StandardMacros.IsValid` (`self.ActiveGameState`)
    (:`Is Valid`
      (`GameState_Base.Tick` (`self.ActiveGameState`) DeltaSeconds))))

(event `InputAction|Primary`
  (params (Key :type "Key Structure"))
  (:`Released`
    (if (`self.bAllowInput`)
      (`/Engine/EditorBlueprintResources/StandardMacros.IsValid` (`self.ActiveGameState`)
        (:`Is Valid`
          (`GameState_Base.PrimaryAction` (`self.ActiveGameState`)))))))

(event `InputAction|Secondary`
  (params (Key :type "Key Structure"))
  (:`Released`
    (if (`self.IsGameStateValidAndInputAllowed?`)
      (`GameState_Base.SecondaryAction` (`self.ActiveGameState`)))))

(event `InputAction|Cancel`
  (params (Key :type "Key Structure"))
  (:`Released`
    (if (`self.IsGameStateValidAndInputAllowed?`)
      (`GameState_Base.Cancel` (`self.ActiveGameState`)))))

(event `Key|Q`
  (params (Key :type "Key Structure"))
  (:`Released`
    (if (`self.IsGameStateValidAndInputAllowed?`)
      (`GameState_Base.RotateLeftAction` (`self.ActiveGameState`)))))

(event `Key|E`
  (params (Key :type "Key Structure"))
  (:`Released`
    (if (`self.IsGameStateValidAndInputAllowed?`)
      (`GameState_Base.RotateRightAction` (`self.ActiveGameState`)))))

(fn `CreateAndShowGameUI`
  (bind _returnvalue (`|CreateWidget` "/Game/UI/WBP_GameUI.WBP_GameUI_C"))
  (`UserWidget.AddToViewport` _returnvalue 0)
  (set `self.GameUI` _returnvalue))

(fn `HideGameUI`
  (`Widget.RemoveFromParent` (`self.GameUI`)))

(fn `IsGameStateValidAndInputAllowed?`
  (returns (ReturnValue :type Boolean))
  (return (and (`self.bAllowInput`) (`KismetSystemLibrary.IsValid` (`self.ActiveGameState`)))))

(fn `Open Build Mode`
  (params (PlaceableData :type "GridObjectData Object Reference"))
  (bind _returnvalue (`|GenericCreateObject` "/Game/Core/GameStates/BP_GameState_Build.BP_GameState_Build_C" PlaceableData))
  (`self.SwitchGameState` _returnvalue))

(fn `SwitchGameState`
  (params (NewGameState :type "GameState_Base Object Reference"))
  (bind _activegamestate (`self.ActiveGameState`))
  (`/Engine/EditorBlueprintResources/StandardMacros.IsValid` _activegamestate
    (:`Is Valid`
      (`GameState_Base.ExitState` _activegamestate))
    (:`Is Not Valid`
      _))
  (bind _output_get (set `self.ActiveGameState` NewGameState))
  (`GameState_Base.EnterState` _output_get))

(fn `UserConstructionScript`)