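; Player controller for the main menu that shows the mouse cursor and handles the intro fade-in.
; On BeginPlay it holds the screen black, then starts a timed camera fade in from black.
; After the fade delay it creates WBP_MainMenu and adds it to the viewport.
; Tick only calls the parent, and leftover logic for yawing the pawn's spring arm from axis input is disconnected.
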(event `self.ReceiveBeginPlay`
  (bind _returnvalue (`GameplayStatics.GetPlayerCameraManager` 0))
  (set `self.bShowMouseCursor` true)
  (`PlayerCameraManager.SetManualCameraFade` :`self` _returnvalue :`InFadeAmount` 1.0)
  (`KismetSystemLibrary.Delay` 1.0)
  (`PlayerCameraManager.StartCameraFade` :`self` _returnvalue :`FromAlpha` 1.0 :`Duration` 2.0)
  (`KismetSystemLibrary.Delay` 2.0)
  (bind _returnvalue_2 (`|CreateWidget` "/Game/UI/WBP_MainMenu.WBP_MainMenu_C"))
  (`UserWidget.AddToViewport` _returnvalue_2 0))

(event `self.ReceiveTick`
  (params (DeltaSeconds :type "Float (single-precision)"))
  (`parent.ReceiveTick` DeltaSeconds))

(event `InputAction|Primary`
  (params (Key :type "Key Structure")))

(event `InputAction|Secondary`
  (params (Key :type "Key Structure")))

(event `InputAction|Cancel`
  (params (Key :type "Key Structure")))

(fn `UserConstructionScript`)