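; Placement rule that allows grid placement only when a neighbouring tile holds an object from one of the matching grid object groups.
; GetValidTilesFromArea checks the grid actors on each candidate neighbour tile and compares their groups against MatchingGroups.
; It rewrites the neighbour list with the matches, adding a tile once per matching actor.
; With no match, it clears the valid tile output and returns false.
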(fn `GetValidTilesFromArea`
  (params (ValidTilesOut :type "Array of IntPoint Structure (by ref)") (ValidNeighbouringTiles :type "Array of IntPoint Structure (by ref)") (GridInstance :type "Grid Object Reference"))
  (returns (ReturnValue :type Boolean))
  (locals (Result :type "Array of IntPoint Structure"))
  (for _array_element ValidNeighbouringTiles
    (for _array_element_2 (`Grid.GetGridActorsAt` (`local.GridInstance`) _array_element)
      (if (`/Game/BP_FunctionLibrary.CompareGridGroupType` (`GridObjectData.MyGridObjectGroups` (`GridObject.GridObjectData` _array_element_2)) (`self.MatchingGroups`))
        (`KismetArrayLibrary.Array_Add` (`local.Result`) _array_element))))
  (`KismetArrayLibrary.Array_Clear` (`local.ValidNeighbouringTiles`))
  (for _array_element_3 (`local.Result`)
    (`KismetArrayLibrary.Array_Add` (`local.ValidNeighbouringTiles`) _array_element_3))
  (if (> (`KismetArrayLibrary.Array_Length` (`local.ValidNeighbouringTiles`)) 0)
    (return true)
    (else
      (`KismetArrayLibrary.Array_Clear` (`local.ValidTilesOut`))
      (return false))))