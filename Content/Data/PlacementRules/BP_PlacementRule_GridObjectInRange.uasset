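; Placement rule that requires certain grid object types to be present among the neighbouring tiles supplied to it.
; GetValidTilesFromArea queries the grid instance for actors on each tile and matches their exact class against GridObjectTypes, printing each match as debug output.
; It narrows the neighbouring tiles to those matches and passes if any remain, otherwise it clears the valid output tiles and fails.
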(fn `GetValidTilesFromArea`
  (params (ValidTilesOut :type "Array of IntPoint Structure (by ref)") (ValidNeighbouringTiles :type "Array of IntPoint Structure (by ref)") (GridInstance :type "Grid Object Reference"))
  (returns (ReturnValue :type Boolean))
  (locals (Result :type "Array of IntPoint Structure"))
  (for _array_element ValidNeighbouringTiles
    (for _array_element_2 (`Grid.GetGridActorsAt` (`local.GridInstance`) _array_element)
      (bind _returnvalue (`GameplayStatics.GetObjectClass` _array_element_2))
      (if (`KismetArrayLibrary.Array_Contains` (`self.GridObjectTypes`) _returnvalue)
        (`KismetSystemLibrary.PrintString` (`KismetSystemLibrary.GetClassDisplayName` _returnvalue))
        (`KismetArrayLibrary.Array_Add` (`local.Result`) _array_element))))
  (`KismetArrayLibrary.Array_Clear` (`local.ValidNeighbouringTiles`))
  (for _array_element_3 (`local.Result`)
    (`KismetArrayLibrary.Array_Add` (`local.ValidNeighbouringTiles`) _array_element_3))
  (if (> (`KismetArrayLibrary.Array_Length` (`local.ValidNeighbouringTiles`)) 0)
    (return true)
    (else
      (`KismetArrayLibrary.Array_Clear` (`local.ValidTilesOut`))
      (return false))))