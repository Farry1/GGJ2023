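; A placement rule that grades where an object can be placed by the number of nearby shallow-rooted trees.
; CanBePlaced reads overlapping actors from the owner's BP_OverlapCheckComponent and counts those that cast to BP_PlaceableObject_Tree and lack deep roots.
; It returns Fail below MinNumber, Perfect when a passing count equals PerfectNumber, and Passed otherwise.
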(fn `CanBePlaced`
  (params (OwningActor :type "Actor Object Reference"))
  (returns (ReturnValue :type "EPlacementRuleResult Enum"))
  (set `self.RootsCount` 0)
  (for _array_element (`/Game/Components/BP_OverlapCheckComponent.GetOverlappingActors` (`Actor.GetComponentByClass` OwningActor "/Game/Components/BP_OverlapCheckComponent.BP_OverlapCheckComponent_C"))
    (bind _asbp_placeable_object_tree (cast `/Game/PlaceableObjects/Trees/BP_PlaceableObject_Tree` _array_element))
    (if (not (`/Game/PlaceableObjects/Trees/BP_PlaceableObject_Tree.bHasDeepRoots` _asbp_placeable_object_tree))
      (`/Engine/EditorBlueprintResources/StandardMacros.IncrementInt` (`self.RootsCount`))))
  (if (>= (`self.RootsCount`) (`self.MinNumber`))
    (if (== (`self.RootsCount`) (`self.PerfectNumber`))
      (return "Perfect")
      (else
        (return "Passed")))
    (else
      (return "Fail"))))