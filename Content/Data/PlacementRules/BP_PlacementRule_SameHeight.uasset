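; A grid placement rule that checks whether every tile in a candidate area sits at the same terrain height.
; It raycasts the terrain at each tile, then keeps hits whose Z lies within a small tolerance of the first hit's.
; It returns true if all tiles pass; otherwise it narrows the valid tile list to the matches, or empties it without hits, and returns false.
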(fn `GetValidTilesFromArea`
  (params (ValidTilesOut :type "Array of IntPoint Structure (by ref)") (AdditionalTilesOut :type "Array of IntPoint Structure (by ref)") (GridInstance :type "Grid Object Reference"))
  (returns (ReturnValue :type Boolean))
  (locals (InitialCount :type Integer :default 0) (WorldLocations :type "Array of Vector Structure") (InitialHeight :type "Float (double-precision)") (CompareLocation :type "Vector Structure") (Result :type "Array of IntPoint Structure"))
  (bind _worldlocations (`local.WorldLocations`))
  (set `local.InitialCount` (`KismetArrayLibrary.Array_Length` ValidTilesOut))
  (for _array_element ValidTilesOut
    (bind (_result _location) (`/Game/BP_FunctionLibrary.RaycastTerrainAtGridPosition` GridInstance _array_element))
    (if _result
      (`KismetArrayLibrary.Array_Add` (`local.WorldLocations`) _location)))
  (if (> (`KismetArrayLibrary.Array_Length` (`local.WorldLocations`)) 0)
    (set `local.CompareLocation` (`|GetArrayItem` _worldlocations))
    (for _array_element_2 _worldlocations
      (if (`KismetMathLibrary.NearlyEqual_FloatFloat` (.z _array_element_2) (.z (`local.CompareLocation`)) 10.0)
        (`KismetArrayLibrary.Array_Add` (`local.Result`) (`Grid.GetGridPosition` (`local.GridInstance`) _array_element_2))))
    (if (== (`KismetArrayLibrary.Array_Length` (`local.Result`)) (`local.InitialCount`))
      (return true)
      (else
        (`KismetArrayLibrary.Array_Clear` (`local.ValidTilesOut`))
        (for _array_element_3 (`local.Result`)
          (`KismetArrayLibrary.Array_Add` (`local.ValidTilesOut`) _array_element_3))
        (return false)))
    (else
      (`KismetArrayLibrary.Array_Clear` (`local.ValidTilesOut`))
      (return false))))