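; BP_GridObject_Base is a base Blueprint for objects that occupy cells on a grid and can award points.
; It derives occupying and neighbouring cells from scene components tagged "OccupyingTile" or "Neighbour", converting their world locations through the grid instance.
; Scoring adds points to player 0's progression component in proportion to the actors overlapping its overlap check component.
; The placement event is an empty stub.
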(event `self.ReceiveBeginPlay`
  (`parent.ReceiveBeginPlay`))

(event `self.ReceiveTick`
  (params (DeltaSeconds :type "Float (single-precision)"))
  (`parent.ReceiveTick` DeltaSeconds))

(event `OnBeingPlaced`)

(fn `CalculateAndAddPoints`
  (`/Game/Components/BP_ProgressionComponent.AddPoints` (`self.GetComponentByClass` (`GameplayStatics.GetPlayerController` 0) "/Game/Components/BP_ProgressionComponent.BP_ProgressionComponent_C") (* (`KismetArrayLibrary.Array_Length` (`/Game/Components/BP_OverlapCheckComponent.GetOverlappingActors` (`self.BP_OverlapCheckComponent`))) 25)))

(fn `GetCellsByTag`
  (params (Tag :type Name))
  (returns (Cells :type "Array of IntPoint Structure"))
  (locals (Result :type "Array of IntPoint Structure"))
  (for _array_element (`self.GetComponentsByTag` "/Script/Engine.ActorComponent" Tag)
    (bind _asscene_component (cast `SceneComponent` _array_element))
    (`KismetArrayLibrary.Array_Add` (`local.Result`) (`Grid.GetGridPosition` (`StaticHelpers.GetGridInstance` self) (`SceneComponent.K2_GetComponentLocation` _asscene_component))))
  (return (`local.Result`)))

(fn `GetNeighbouringCells`
  (returns (ReturnValue :type "Array of IntPoint Structure"))
  (`parent.GetNeighbouringCells`)
  (return (`self.GetCellsByTag` "Neighbour")))

(fn `GetOccupyingCells`
  (returns (ReturnValue :type "Array of IntPoint Structure"))
  (`parent.GetOccupyingCells`)
  (return (`self.GetCellsByTag` "OccupyingTile")))

(fn `UserConstructionScript`)