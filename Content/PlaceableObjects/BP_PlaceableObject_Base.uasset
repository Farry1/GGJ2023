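; Base actor for placeable objects that validates placement and awards progression points when placed.
; CanBePlaced allows placement only when the Mesh overlaps no actor other than itself.
; OnBeingPlaced counts actors overlapping the separate BPOverlapCheckComponent and adds points proportional to that count to the BP_ProgressionComponent on the first player controller.
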(event `OnBeingPlaced`
  (`self.CalculateAndAddPoints`))

(fn `CalculateAndAddPoints`
  (`/Game/Components/BP_ProgressionComponent.AddPoints` (`self.GetComponentByClass` (`GameplayStatics.GetPlayerController` 0) "/Game/Components/BP_ProgressionComponent.BP_ProgressionComponent_C") (* (`KismetArrayLibrary.Array_Length` (`/Game/Components/BP_OverlapCheckComponent.GetOverlappingActors` (`self.BP_OverlapCheckComponent`))) 25)))

(fn `CanBePlaced`
  (returns (Result :type Boolean))
  (for _array_element (`PrimitiveComponent.GetOverlappingActors` (`self.Mesh`) null)
    (if (!= _array_element self)
      (return false)))
  (return true))

(fn `UserConstructionScript`)