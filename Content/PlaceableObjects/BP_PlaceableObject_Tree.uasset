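; BP_PlaceableObject_Tree is a tree placeable object that animates a decal when it is placed in the world.
; On BeginPlay it creates a dynamic material instance for its decal and sets the RadiusMultiplier parameter to zero.
; When placed, a timeline drives RadiusMultiplier from its Timer track, animating the decal's radius.
; Other behaviour is left to the parent placeable-object class.
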(event `self.ReceiveBeginPlay`
  (`parent.ReceiveBeginPlay`)
  (bind _returnvalue (`KismetMaterialLibrary.CreateDynamicMaterialInstance` (`DecalComponent.GetDecalMaterial` (`self.Decal`))))
  (`DecalComponent.SetDecalMaterial` (`self.Decal`) _returnvalue)
  (set `self.DecalMaterial` _returnvalue)
  (`MaterialInstanceDynamic.SetScalarParameterValue` (`self.DecalMaterial`) "RadiusMultiplier" 0.0))

(event `self.ReceiveTick`
  (params (DeltaSeconds :type "Float (single-precision)"))
  (`parent.ReceiveTick` DeltaSeconds))

(event `self.OnBeingPlaced`
  (`parent.OnBeingPlaced`)
  (bind (_direction _timer) (`Timeline|Timeline_0` :!via `PlayFromStart`)
    (:`Update`
      (`MaterialInstanceDynamic.SetScalarParameterValue` (`self.DecalMaterial`) "RadiusMultiplier" _timer))))

(fn `UserConstructionScript`
  (`parent.UserConstructionScript`))