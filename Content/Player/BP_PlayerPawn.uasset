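; Player pawn Blueprint that rotates its spring arm camera around the yaw axis in timed, eased or linear steps.
; RotateCamera adds the given direction to the stored yaw, and a timeline lerps the arm to that target, keeping pitch and roll.
; A flag blocks timeline restarts mid-turn, though new calls still overwrite the target.
; The stored yaw updates when the turn finishes.
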(event `RotateCamera`
  (params (Direction :type "Float (double-precision)"))
  (bind _springarm (`self.SpringArm`))
  (bind (_relativerotation_roll _relativerotation_pitch) (`KismetMathLibrary.BreakRotator` (`SceneComponent.RelativeRotation` _springarm)))
  (set `self.TargetRotation` (+ Direction (`self.CurrentCameraRotation`)))
  (if (not (`self.bIsRotating`))
    (set `self.bIsRotating` true)
    (bind (_direction _camerarotation) (`Timeline|RotationTimeline` :!via `PlayFromStart`)
      (:`Update`
        (`SceneComponent.K2_SetRelativeRotation` _springarm (`KismetMathLibrary.MakeRotator` _relativerotation_roll _relativerotation_pitch (`KismetMathLibrary.Lerp` (`self.CurrentCameraRotation`) (`self.TargetRotation`) _camerarotation)) false false))
      (:`Finished`
        (set `self.bIsRotating` false)
        (set `self.CurrentCameraRotation` (`self.TargetRotation`))))))

(fn `UserConstructionScript`)